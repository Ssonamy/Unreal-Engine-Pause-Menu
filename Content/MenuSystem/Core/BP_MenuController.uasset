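; BP_MenuController manages the game's menus: main menu, settings, start, resume and quit.
; On BeginPlay it loads SaveSlot1 and shows the main menu only if that succeeds.
; SwitchWidget swaps the current widget by menu state, passes it controller and save references, and sets pause and input mode, while HandleBack uses the previous state.
; Pause widget creation is unwired, and Tick forces the cursor visible.
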(event `self.ReceiveBeginPlay`
  (`self.Init`))

(event `self.ReceiveTick`
  (params (DeltaSeconds :type "Float (single-precision)"))
  (set `PlayerController.bShowMouseCursor` true (`GameplayStatics.GetPlayerController` 0)))

(fn `HandleBack`
  (switch `/Game/MenuSystem/Core/Enums/EMenuState` (cast `/Game/MenuSystem/Core/Enums/EMenuState` (`self.PreviousMenuState`))
    (:`NewEnumerator0`
      (`self.ShowMainMenu` :!label _label))
    (:`NewEnumerator1`
      (goto _label))
    (:`NewEnumerator2`
      (`self.ShowSettings`))
    (:`NewEnumerator3`
      (`self.ShowPauseMenu`))))

(fn `Init`
  (bind _returnvalue (`GameplayStatics.LoadGameFromSlot` "SaveSlot1"))
  (bind _asbp_save_game_data (cast `/Game/MenuSystem/Data/BP_SaveGameData` _returnvalue)
    (:`then`
      (set `self.SaveGameData` _asbp_save_game_data)
      (`self.ShowMainMenu`)
      (`KismetSystemLibrary.PrintString` "GAME IS STILL RUNNING AFTER 5 SECONDS"))
    (:`CastFailed`
      (bind _returnvalue_2 (`|GenericCreateObject` "/Game/MenuSystem/Data/BP_SaveGameData.BP_SaveGameData_C")))))

(fn `QuitGame`
  (`KismetSystemLibrary.QuitGame` (`GameplayStatics.GetPlayerController` 0) "Quit"))

(fn `ResumeGame`
  (bind _returnvalue (`GameplayStatics.GetPlayerController` 0))
  (if (`KismetSystemLibrary.IsValid` (`self.CurrentWidget`))
    (`Widget.RemoveFromParent` (`self.CurrentWidget`)))
  (set `self.CurrentWidget` null)
  (`GameplayStatics.SetGamePaused` false)
  (`WidgetBlueprintLibrary.SetInputMode_GameOnly` _returnvalue)
  (set `PlayerController.bShowMouseCursor` true _returnvalue))

(fn `ShowMainMenu`
  (set `self.PreviousMenuState` (`self.CurrentMenuState`))
  (`self.SwitchWidget` 1))

(fn `ShowPauseMenu`
  (set `self.PreviousMenuState` (`self.CurrentMenuState`))
  (`self.SwitchWidget` 3))

(fn `ShowSettings`
  (set `self.PreviousMenuState` (`self.CurrentMenuState`))
  (`self.SwitchWidget` 2))

(fn `StartGame`
  (bind _returnvalue (`GameplayStatics.GetPlayerController` 0))
  (if (`KismetSystemLibrary.IsValid` (`self.CurrentWidget`))
    (`Widget.RemoveFromParent` (`self.CurrentWidget`)))
  (set `self.CurrentWidget` null)
  (`GameplayStatics.SetGamePaused` false)
  (`WidgetBlueprintLibrary.SetInputMode_UIOnlyEx` _returnvalue null "LockAlways")
  (set `PlayerController.bShowMouseCursor` true _returnvalue)
  (`GameplayStatics.OpenLevel` "L_GameLevel"))

(fn `SwitchWidget`
  (params (NewState :type Byte :default 0))
  (locals (CreatedWidget :type "UserWidget Object Reference") (NewLocalVar :type "/Game/MenuSystem/Core/BP_MenuController Object Reference"))
  (bind _returnvalue (`GameplayStatics.GetPlayerController` 0))
  (bind _returnvalue_2 (`GameplayStatics.GetPlayerController` 0))
  (bind _returnvalue_3 (`GameplayStatics.GetPlayerController` 0))
  (bind _returnvalue_4 (`GameplayStatics.GetPlayerController` 0))
  (if (`KismetSystemLibrary.IsValid` (`self.CurrentWidget`))
    (`Widget.RemoveFromParent` (`self.CurrentWidget`)))
  (set `self.CurrentWidget` null)
  (switch `/Game/MenuSystem/Core/Enums/EMenuState` (cast `/Game/MenuSystem/Core/Enums/EMenuState` NewState)
    (:`NewEnumerator1`
      (bind _returnvalue_5 (`|CreateWidget` (`GameplayStatics.GetObjectClass` (`self.MainMenuClass`))))
      (set `local.CreatedWidget` _returnvalue_5)
      (if (`KismetSystemLibrary.IsValid` (`local.CreatedWidget`))
        (bind _aswbp_main_menu (cast `/Game/MenuSystem/Widgets/WBP_MainMenu` (`local.CreatedWidget`)))
        (set `/Game/MenuSystem/Widgets/WBP_MainMenu.MenuControllerRef` self _aswbp_main_menu)
        (`UserWidget.AddToViewport` (`local.CreatedWidget`) 100)
        (set `self.CurrentWidget` (`local.CreatedWidget`))
        (set `self.CurrentMenuState` NewState)
        (switch `/Game/MenuSystem/Core/Enums/EMenuState` (cast `/Game/MenuSystem/Core/Enums/EMenuState` NewState) :!label _label
          (:`NewEnumerator1`
            (`GameplayStatics.SetGamePaused` false)
            (`WidgetBlueprintLibrary.SetInputMode_UIOnlyEx` _returnvalue_3 null)
            (set `PlayerController.bShowMouseCursor` true _returnvalue_3))
          (:`NewEnumerator2`
            (if (== (`self.PreviousMenuState`) 3)
              (`GameplayStatics.SetGamePaused` true)
              (`WidgetBlueprintLibrary.SetInputMode_UIOnlyEx` _returnvalue_4 (`self.CurrentWidget`))
              (set `PlayerController.bShowMouseCursor` true _returnvalue_4)
              (else
                (`GameplayStatics.SetGamePaused` false)
                (`WidgetBlueprintLibrary.SetInputMode_UIOnlyEx` _returnvalue (`self.CurrentWidget`))
                (set `PlayerController.bShowMouseCursor` true _returnvalue))))
          (:`NewEnumerator3`
            (`GameplayStatics.SetGamePaused` true)
            (`WidgetBlueprintLibrary.SetInputMode_UIOnlyEx` _returnvalue_2 (`self.CurrentWidget`))
            (set `PlayerController.bShowMouseCursor` true _returnvalue_2)))))
    (:`NewEnumerator2`
      (bind _returnvalue_6 (`|CreateWidget` (`GameplayStatics.GetObjectClass` (`self.SettingsMenuClass`))))
      (set `local.CreatedWidget` _returnvalue_6)
      (if (`KismetSystemLibrary.IsValid` (`local.CreatedWidget`))
        (bind _aswbp_settings (cast `/Game/MenuSystem/Widgets/WBP_Settings` (`local.CreatedWidget`)))
        (set `/Game/MenuSystem/Widgets/WBP_Settings.MenuControllerRef` self _aswbp_settings)
        (set `/Game/MenuSystem/Widgets/WBP_Settings.SaveData` (`self.SaveGameData`) _aswbp_settings)
        (`UserWidget.AddToViewport` (`local.CreatedWidget`) 100)
        (set `self.CurrentWidget` (`local.CreatedWidget`))
        (set `self.CurrentMenuState` NewState)
        (goto _label)
        (else
          (`KismetSystemLibrary.PrintString` "its wrong"))))))

(fn `SwitchWidget_1`
  (params (Byte :type Byte))
  (locals (CreatedWidget :type "UserWidget Object Reference"))
  (if (`KismetSystemLibrary.IsValid` (`self.CurrentWidget`))
    (`Widget.RemoveFromParent` (`self.CurrentWidget`)))
  (set `self.CurrentWidget` null)
  (switch `/Game/MenuSystem/Core/Enums/EMenuState` (cast `/Game/MenuSystem/Core/Enums/EMenuState` Byte)))

(fn `UserConstructionScript`)